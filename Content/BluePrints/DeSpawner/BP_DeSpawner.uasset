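; BP_DeSpawner is an actor that trails the player at a fixed offset along negative world X, apparently as a despawn point.
; On BeginPlay it caches a TriggerVolume as KillZoneVolume and starts a looping timer.
; The timer teleports it behind player 0 without sweeping.
; On overlap with any actor except KillZoneVolume, it destroys itself, not the overlapping actor.
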(event `self.ReceiveBeginPlay`
  (bind _returnvalue (`GameplayStatics.GetActorOfClass` "/Script/Engine.TriggerVolume"))
  (set `self.KillZoneVolume` _returnvalue)
  (`KismetSystemLibrary.K2_SetTimerDelegate` (delegate `UpdatePosition`) 0.1 true))

(event `UpdatePosition`
  (`self.K2_SetActorLocation` (- (`self.K2_GetActorLocation` (`GameplayStatics.GetPlayerCharacter` 0)) (1000.0 0.0 0.0)) false true))

(event `self.ReceiveActorBeginOverlap`
  (params (OtherActor :type "Actor Object Reference"))
  (if (not (== OtherActor (`self.KillZoneVolume`)))
    (`self.K2_DestroyActor`)))

(fn `UserConstructionScript`)