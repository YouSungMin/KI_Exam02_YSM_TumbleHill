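; BP_SpawnerTest is a test spawner that periodically spawns random tumble actors at a set of spawn points.
; A looping timer started on BeginPlay fires every two seconds and calls TumbleActorSpawn once per entry in the Spawnpoint array.
; Each call spawns a random class from TumbleActors at the current point's transform, ignoring collisions, then advances a wrapping index so every point gets one actor per wave.
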(event `self.ReceiveBeginPlay`
  (bind _returnvalue (`KismetSystemLibrary.K2_SetTimerDelegate` (delegate `ActorsSpawn`) 2.0 true))
  (set `self.SpawnTimerHandle` _returnvalue))

(event `ActorsSpawn`
  (for _ (range 1 (+ (`KismetArrayLibrary.Array_Length` (`self.Spawnpoint`)) 1))
    (`self.TumbleActorSpawn`)))

(event `IncreaseSpawnPointIndex`
  (bind _result (`/Engine/EditorBlueprintResources/StandardMacros.IncrementInt` (`self.SpawnpointIndex`))
    (:`  `
      (set `self.SpawnpointIndex` (mod _result (`KismetArrayLibrary.Array_Length` (`self.Spawnpoint`)))))))

(fn `UserConstructionScript`)