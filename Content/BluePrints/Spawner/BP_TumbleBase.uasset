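; BP_TumbleBase is a physics-driven tumbling hazard, apparently a base for variants, that damages the player on contact.
; A looping timer started at BeginPlay checks the mesh's speed and, when slow, adds randomized mass-independent impulses along world -X and upward, plus random spin, to keep it rolling.
; Hitting the player character applies damage through a DoOnce that is never reset, so each instance hurts only once.
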(event `self.ReceiveBeginPlay`
  (bind _returnvalue (`KismetSystemLibrary.K2_SetTimer` null "PushIfStopped" 0.1 true))
  (set `self.MoveTimerHandle` _returnvalue)
  (`self.PushIfStopped`))

(event `self.ReceiveHit`
  (params (MyComp :type "PrimitiveComponent Object Reference") (Other :type "Actor Object Reference") (OtherComp :type "PrimitiveComponent Object Reference") (bSelfMoved :type Boolean) (HitLocation :type "Vector Structure") (HitNormal :type "Vector Structure") (NormalImpulse :type "Vector Structure") (Hit :type "HitResult Structure (by ref)"))
  (if (== Other (`GameplayStatics.GetPlayerCharacter` 0))
    (`/Engine/EditorBlueprintResources/StandardMacros.DoOnce` false
      (:`Completed`
        (`GameplayStatics.ApplyDamage` Other (`self.Damage`))))))

(fn `PushIfStopped`
  (bind _returnvalue (`KismetMathLibrary.RandomFloatInRange` -360.0 360.0))
  (bind _staticmesh (`self.StaticMesh`))
  (bind _returnvalue_2 (`PrimitiveComponent.GetPhysicsLinearVelocity` (`self.StaticMesh`) "None"))
  (if (< (`KismetMathLibrary.VSize` _returnvalue_2) 1000.0)
    (`PrimitiveComponent.AddImpulse` _staticmesh (`KismetMathLibrary.MakeVector` (`KismetMathLibrary.RandomFloatInRange` -1000.0 -500.0) 0.0 (`KismetMathLibrary.RandomFloatInRange` 100.0 200.0)) "None" true)
    (`PrimitiveComponent.AddAngularImpulseInDegrees` _staticmesh (`KismetMathLibrary.MakeVector` _returnvalue 0.0 _returnvalue) "None" true)))

(fn `UserConstructionScript`
  (`parent.UserConstructionScript`))