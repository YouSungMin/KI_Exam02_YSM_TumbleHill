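; BP_Tumble_LuckyBox1 is a lucky box that gives the player a random effect on hit.
; Its Hit event casts the other actor to BP_Player, then switches on a random index from 3 to MaxItemIndex to call that player's Apply function and destroy the box.
; With the minimum at 3, speed boost, invincibility and screen clear are never rolled, leaving movement, jump, shrink and paper-thin effects.
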(event `self.ReceiveHit`
  (params (MyComp :type "PrimitiveComponent Object Reference") (Other :type "Actor Object Reference") (OtherComp :type "PrimitiveComponent Object Reference") (bSelfMoved :type Boolean) (HitLocation :type "Vector Structure") (HitNormal :type "Vector Structure") (NormalImpulse :type "Vector Structure") (Hit :type "HitResult Structure (by ref)"))
  (bind _asbp_player (cast `/Game/BluePrints/Player/BP_Player` Other))
  (switch `int` (`KismetMathLibrary.RandomIntegerInRange` 3 (`self.MaxItemIndex`))
    (:`0`
      (`/Game/BluePrints/Player/BP_Player.ApplySpeedBoost` _asbp_player))
    (:`1`
      (`/Game/BluePrints/Player/BP_Player.ApplyInvincibility` _asbp_player))
    (:`2`
      (`/Game/BluePrints/Player/BP_Player.ApplyClearScreen` _asbp_player))
    (:`3`
      (`/Game/BluePrints/Player/BP_Player.ApplySlowMovement` _asbp_player))
    (:`4`
      (`/Game/BluePrints/Player/BP_Player.ApplyFastMovement` _asbp_player))
    (:`5`
      (`/Game/BluePrints/Player/BP_Player.ApplySuperJump` _asbp_player))
    (:`6`
      (`/Game/BluePrints/Player/BP_Player.ApplyPlayerShrink` _asbp_player))
    (:`7`
      (`/Game/BluePrints/Player/BP_Player.ApplyPaperThinEffect` _asbp_player)))
  (`self.K2_DestroyActor`))

(fn `UserConstructionScript`
  (`parent.UserConstructionScript`))