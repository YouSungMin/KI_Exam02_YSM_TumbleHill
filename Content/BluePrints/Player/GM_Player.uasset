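; GM_Player is the game mode that sets up difficulty and handles player respawn and game end.
; On BeginPlay it caches the game instance and finds BP_Spawner, then sets the spawner's respawn cycle from the selected difficulty and starts it.
; RespawnPlayer spawns the player class and has the first controller possess it.
; Game over and game clear handlers only print debug strings.
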(event `ApplyGameDifficulty`
  (bind _gamespawner (`self.GameSpawner`))
  (`/Engine/EditorBlueprintResources/StandardMacros.IsValid` (`self.GameSpawner`)
    (:`Is Valid`
      (switch `/Game/BluePrints/Enums/E_Difficulty` (`/Game/BluePrints/BP_GameInstance.SelectedDifficulty` (`self.GameInstance`))
        (:`NewEnumerator0`
          (set `/Game/BluePrints/Spawner/BP_Spawner.RespawnCycle` 2.5 _gamespawner))
        (:`NewEnumerator1`
          (set `/Game/BluePrints/Spawner/BP_Spawner.RespawnCycle` 1.5 _gamespawner)))
      (`/Game/BluePrints/Spawner/BP_Spawner.StartSpawner` _gamespawner))))

(event `self.ReceiveBeginPlay`
  (bind _returnvalue (`GameplayStatics.GetGameInstance`))
  (`/Engine/EditorBlueprintResources/StandardMacros.IsValid` _returnvalue
    (:`Is Valid`
      (bind _asbp_game_instance (cast `/Game/BluePrints/BP_GameInstance` _returnvalue))
      (set `self.GameInstance` _asbp_game_instance)
      (bind _returnvalue_2 (`GameplayStatics.GetActorOfClass` "/Game/BluePrints/Spawner/BP_Spawner.BP_Spawner_C"))
      (set `self.GameSpawner` _returnvalue_2)
      (`self.ApplyGameDifficulty`))))

(event `RespawnPlayer`
  (bind _returnvalue (`|SpawnActorFromClass` (`self.PlayerClass`) (`KismetMathLibrary.MakeTransform` (0.0 0.0 0.0)) "Undefined" "MultiplyWithRoot" null null))
  (bind `_as캐릭터` (cast `Character` _returnvalue))
  (`Controller.Possess` (`GameplayStatics.GetPlayerController` 0) `_as캐릭터`))

(event `HandleGameOver`
  (`KismetSystemLibrary.PrintString` "GameOver"))

(event `HandleGameClear`
  (`KismetSystemLibrary.PrintString` "GameClear"))

(fn `UserConstructionScript`)