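; In-game game mode that sets difficulty, tracks player lives and decides game over or clear.
; On BeginPlay it caches the game instance, player controller and level spawner, then sets the spawner's respawn cycle from the selected difficulty and starts it.
; Losing a life decrements the controller's life count, then either respawns and possesses a new character after a delay or ends the game.
; Win and loss results are forwarded to the player controller.
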(event `ApplyGameDifficulty`
  (bind _gamespawner (`self.GameSpawner`))
  (`/Engine/EditorBlueprintResources/StandardMacros.IsValid` (`self.GameSpawner`)
    (:`Is Valid`
      (switch `/Game/BluePrints/Enums/E_Difficulty` (`/Game/BluePrints/BP_GameInstance.SelectedDifficulty` (`self.GameInstance`))
        (:`NewEnumerator0`
          (set `/Game/BluePrints/Spawner/BP_Spawner.RespawnCycle` 2.5 _gamespawner))
        (:`NewEnumerator1`
          (set `/Game/BluePrints/Spawner/BP_Spawner.RespawnCycle` 1.5 _gamespawner)))
      (`/Game/BluePrints/Spawner/BP_Spawner.StartSpawner` _gamespawner))))

(event `self.ReceiveBeginPlay`
  (bind _returnvalue (`GameplayStatics.GetGameInstance`))
  (`/Engine/EditorBlueprintResources/StandardMacros.IsValid` _returnvalue
    (:`Is Valid`
      (bind _asbp_game_instance (cast `/Game/BluePrints/BP_GameInstance` _returnvalue))
      (set `self.GameInstance` _asbp_game_instance)
      (bind _aspc_player_controller (cast `/Game/BluePrints/Player/PC_PlayerController` (`GameplayStatics.GetPlayerController` 0)))
      (set `self.PlayerController` _aspc_player_controller)
      (bind _returnvalue_2 (`GameplayStatics.GetActorOfClass` "/Game/BluePrints/Spawner/BP_Spawner.BP_Spawner_C"))
      (set `self.GameSpawner` _returnvalue_2)
      (`self.ApplyGameDifficulty`))))

(event `RespawnPlayer`
  (`KismetSystemLibrary.Delay` 2.0)
  (bind _returnvalue (`|SpawnActorFromClass` (`self.PlayerClass`) (`KismetMathLibrary.MakeTransform` (0.0 0.0 0.0)) "Undefined" "MultiplyWithRoot" null null))
  (bind `_as캐릭터` (cast `Character` _returnvalue))
  (`Controller.Possess` (`self.PlayerController`) `_as캐릭터`))

(event `PlayerLifedecrease`
  (bind _playercontroller (`self.PlayerController`))
  (bind _result (`/Engine/EditorBlueprintResources/StandardMacros.DecrementInt` (`/Game/BluePrints/Player/PC_PlayerController.PlayerLife` _playercontroller))
    (:`  `
      (bind _output_get (set `/Game/BluePrints/Player/PC_PlayerController.PlayerLife` _result _playercontroller))
      (if (<= _output_get 0)
        (`self.HandleGameOver`)
        (else
          (`self.RespawnPlayer`))))))

(event `HandleGameOver`
  (`/Game/BluePrints/Player/PC_PlayerController.PlayerGameFinish` (`self.PlayerController`) false))

(event `HandleGameClear`
  (`/Game/BluePrints/Player/PC_PlayerController.PlayerGameFinish` (`self.PlayerController`) true))

(fn `UserConstructionScript`)