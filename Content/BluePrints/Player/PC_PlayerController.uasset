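; Player controller that owns the in-game HUD, the pause menu and the player's health count.
; BeginPlay adds the input mapping and HUD, and the pause input opens the pause widget in UI-only input mode.
; Events handle resume, level restart and return to the title map.
; Each hit decrements health and updates the HUD, then asks GM_Player to respawn the player, or handle game over at zero.
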(event `self.ReceiveBeginPlay`
  (set `self.bShowMouseCursor` false)
  (`WidgetBlueprintLibrary.SetInputMode_GameOnly` (`GameplayStatics.GetPlayerController` 0))
  (`EnhancedInputSubsystemInterface.AddMappingContext` (subsystem `EnhancedInputLocalPlayerSubsystem`) (`self.Mapping Context`) 0 (struct))
  (bind _returnvalue (`|CreateWidget` "/Game/UI/InGame/WBP_InGameHUD.WBP_InGameHUD_C"))
  (bind _output_get (set `self.HudRef` _returnvalue))
  (`UserWidget.AddToViewport` _output_get 0)
  (`self.UpdateHealthUI`)
  (bind _asgm_player (cast `/Game/BluePrints/Player/GM_Player` (`GameplayStatics.GetGameMode`)))
  (set `self.GameMode` _asgm_player))

(event `EnhancedInput|/Game/Input/IA_Puase`
  (params (ActionValue :type Boolean) (ElapsedSeconds :type "Float (double-precision)") (TriggeredSeconds :type "Float (double-precision)") (InputAction :type "InputAction Object Reference" :default "/Game/Input/IA_Puase.IA_Puase"))
  (:`Triggered`
    (if (not (`GameplayStatics.IsGamePaused`))
      (`GameplayStatics.SetGamePaused` true)
      (bind _returnvalue (`|CreateWidget` "/Game/UI/Title/WBP_Pause.WBP_Pause_C"))
      (bind _output_get (set `self.PauseMenuRef` _returnvalue))
      (`UserWidget.AddToViewport` _output_get 0)
      (set `self.bShowMouseCursor` true)
      (`WidgetBlueprintLibrary.SetInputMode_UIOnlyEx` (`GameplayStatics.GetPlayerController` 0) null))))

(event `ResumeGame`
  (bind _pausemenuref (`self.PauseMenuRef`))
  (`/Engine/EditorBlueprintResources/StandardMacros.IsValid` _pausemenuref
    (:`Is Valid`
      (`Widget.RemoveFromParent` _pausemenuref)
      (`GameplayStatics.SetGamePaused` false)
      (set `self.bShowMouseCursor` false)
      (`WidgetBlueprintLibrary.SetInputMode_GameOnly` (`GameplayStatics.GetPlayerController` 0)))))

(event `RestartGame`
  (`GameplayStatics.SetGamePaused` false)
  (bind _returnvalue (`GameplayStatics.GetCurrentLevelName` true))
  (`GameplayStatics.OpenLevel` (`KismetStringLibrary.Conv_StringToName` _returnvalue)))

(event `GoToMainMenu`
  (`GameplayStatics.SetGamePaused` false)
  (`GameplayStatics.OpenLevel` "TitleMap"))

(event `PlayerTookDamage`
  (bind _gamemode (`self.GameMode`))
  (bind _result (`/Engine/EditorBlueprintResources/StandardMacros.DecrementInt` (`self.CurrentHealth`))
    (:`  `
      (set `self.CurrentHealth` _result)
      (`self.UpdateHealthUI`)
      (if (<= (`self.CurrentHealth`) 0)
        (`/Game/BluePrints/Player/GM_Player.HandleGameOver` _gamemode)
        (else
          (`/Game/BluePrints/Player/GM_Player.RespawnPlayer` _gamemode))))))

(fn `UpdateHealthUI`
  (bind _hudref (`self.HudRef`))
  (`/Engine/EditorBlueprintResources/StandardMacros.IsValid` _hudref
    (:`Is Valid`
      (`/Game/UI/InGame/WBP_InGameHUD.UpdateHealthDisplay` _hudref (`self.CurrentHealth`)))))

(fn `UserConstructionScript`)